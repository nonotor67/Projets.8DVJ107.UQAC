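; Puzzle-item spawner that places either a physics cube or a laser cube at its own transform when play begins.
; The CubeCubeLaser flag selects the class in Spawn: BP_PhysicsCube when true, A_laserCube when false.
; Spawner and spawned cube store references to each other, with a separate spawner-side variable for each cube type.
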(event EventBeginPlay
  (CallFunction|Spawn))

(event Collision|EventActorBeginOverlap
  (params (OtherActor :type Actor%20Object%20Reference)))

(event EventTick
  (params (DeltaSeconds :type Float%20%28single-precision%29)))

(fn ConstructionScript)

(fn Spawn
  (bind _returnvalue (Transformation|GetActorTransform))
  (if (Variables|Default|GetCube/CubeLaser)
    (bind _returnvalue_2 (Game|SpawnActorfromClass "/Game/PuzzleItems/Blueprints/BP_PhysicsCube.BP_PhysicsCube_C" _returnvalue "Undefined" "MultiplyWithRoot" 0 0))
    (Variables|Default|SetLinkedCube _returnvalue_2)
    (Variables|/Game/PuzzleItems/Blueprints/BP_PhysicsCube.BP_PhysicsCube_C|SetLinkedSpawner _returnvalue_2 self)
    (else
      (bind _returnvalue_3 (Game|SpawnActorfromClass "/Game/lasers/A_laserCube.A_laserCube_C" _returnvalue "Undefined" "MultiplyWithRoot" 0 "(R=0.000000,G=0.000000,B=0.000000,A=0.000000)" 0 0))
      (Variables|Default|SetLinkedCubeLaser _returnvalue_3)
      (Variables|/Game/lasers/A_laserCube.A_laserCube_C|SetLinkedSpawner _returnvalue_3 self))))