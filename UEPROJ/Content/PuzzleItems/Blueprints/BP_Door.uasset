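; BP_Door is a puzzle door that slides down to open and back up to close through its OpenDoor and CloseDoor events.
; Each event stores the mesh's current relative Z and a target height, plays a sound and restarts a shared Timeline.
; The Timeline linearly interpolates the door between those heights, so a reversal mid-move starts from the current position.
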(event Custom|OpenDoor
  (Variables|Default|SetCurrentHeight (.z (Variables|/Script/Engine.SceneComponent|GetRelativeLocation (Variables|Default|GetDoor))))
  (Variables|Default|SetNewHeight -2.2e+02)
  (Audio|PlaySoundatLocation 0 (Transformation|GetActorLocation) "0, 0, 0" 1.0 1.0 0.0 0 0 0 0)
  (bind _alpha (Timeline|Timeline PlayFromStart)
    (:Update
      (Transformation|SetRelativeLocation (Variables|Default|GetDoor) (Math|Vector|MakeVector 0.0 0.0 (Math|Interpolation|Ease "Linear" _alpha (Variables|Default|GetCurrentHeight) (Variables|Default|GetNewHeight))) false false))))

(event Custom|CloseDoor
  (Variables|Default|SetCurrentHeight (.z (Variables|/Script/Engine.SceneComponent|GetRelativeLocation (Variables|Default|GetDoor))))
  (Variables|Default|SetNewHeight 0.0)
  (Audio|PlaySoundatLocation 0 (Transformation|GetActorLocation) "0, 0, 0" 1.0 1.0 0.0 0 0 0 0)
  (bind _alpha (Timeline|Timeline PlayFromStart)
    (:Update
      (Transformation|SetRelativeLocation (Variables|Default|GetDoor) (Math|Vector|MakeVector 0.0 0.0 (Math|Interpolation|Ease "Linear" _alpha (Variables|Default|GetCurrentHeight) (Variables|Default|GetNewHeight))) false false))))

(event EventBeginPlay)

(event Collision|EventActorBeginOverlap
  (params (OtherActor :type Actor%20Object%20Reference)))

(event EventTick
  (params (DeltaSeconds :type Float%20%28single-precision%29)))

(fn ConstructionScript)